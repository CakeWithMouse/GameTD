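; Player controller that routes input for moving, looking, building and shooting, after applying mouse sensitivity and a starting movement speed on BeginPlay.
; Enhanced Input actions call the matching functions, and Build also alternates two on-screen messages through a FlipFlop.
; Raw keys serve as controls: Up and Down adjust move speed, and holding T enables Freecam.
; LookAround also accumulates CameraRotation, clamping vertical input in the Roll component, and prints the result.
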(event Input|EnhancedActionEvents|EnhancedInputActionShoot
  (params (ActionValue :type Boolean) (ElapsedSeconds :type Float%20%28double-precision%29) (TriggeredSeconds :type Float%20%28double-precision%29) (InputAction :type Input%20Action%20Object%20Reference :default "/Game/Player/Input/StandartInput/Shoot.Shoot"))
  ;[1 1 1] Action
  (Class|AbstractPlayerController|Shoot))

(event Input|EnhancedActionEvents|EnhancedInputActionMove
  (params (ActionValue :type Vector%202D%20Structure) (ElapsedSeconds :type Float%20%28double-precision%29) (TriggeredSeconds :type Float%20%28double-precision%29) (InputAction :type Input%20Action%20Object%20Reference :default "/Game/Player/Input/StandartInput/Move.Move"))
  ;[1 1 1] Move
  (Class|AbstractPlayerController|Move ActionValue))

(event Input|EnhancedActionEvents|EnhancedInputActionLookAround
  (params (ActionValue :type Vector%202D%20Structure) (ElapsedSeconds :type Float%20%28double-precision%29) (TriggeredSeconds :type Float%20%28double-precision%29) (InputAction :type Input%20Action%20Object%20Reference :default "/Game/Player/Input/StandartInput/LookAround.LookAround"))
  (bind (_x _y) (Math|Vector2D|BreakVector2D ActionValue))
  ;[1 1 1] Move
  (Class|AbstractPlayerController|LookAround ActionValue)
  (bind _output_get (Variables|Default|SetCameraRotation (Math|Rotator|MakeRotator (Math|Float|Clamp(Float) (+ _y (.Roll (Math|Rotator|BreakRotator (Variables|Default|GetCameraRotation)))) -1e+01 2e+01) (.Pitch (Math|Rotator|BreakRotator (Variables|Default|GetCameraRotation))) (+ _x (.Yaw (Math|Rotator|BreakRotator (Variables|Default|GetCameraRotation)))))))
  (Development|PrintString (Utilities|String|ToString(Rotator) _output_get)))

(event Input|EnhancedActionEvents|EnhancedInputActionBuild
  (params (ActionValue :type Boolean) (ElapsedSeconds :type Float%20%28double-precision%29) (TriggeredSeconds :type Float%20%28double-precision%29) (InputAction :type Input%20Action%20Object%20Reference :default "/Game/Player/Input/StandartInput/Build.Build"))
  ;[1 1 1] Action
  (Class|AbstractPlayerController|Build 0.0)
  (Utilities|FlowControl|FlipFlop
    (:A
      (Development|PrintString "Enter \"B\" to build here"))
    (:B
      (Development|PrintString "Success"))))

(event EventBeginPlay
  ;[1 1 1] Begin Play
  (bind _returnvalue (Class|AbstractPlayerController|GetMouseSensitivity))
  (Class|AbstractPlayerController|SetMouseSensitivity _returnvalue)
  (Class|AbstractPlayerController|SetMovementSpeed 8e+02))

(event EventTick
  (params (DeltaSeconds :type Float%20%28single-precision%29))
  ;[1 1 1] Tick
)

(event Input|KeyboardEvents|Up
  (params (Key :type Key%20Structure :default "None"))
  ;[1 1 1] Config Speed
  (:Pressed
    (Class|AbstractPlayerController|AddMoveSpeed 2e+02)))

(event Input|KeyboardEvents|Down
  (params (Key :type Key%20Structure :default "None"))
  ;[1 1 1] Config Speed
  (:Pressed
    (Class|AbstractPlayerController|ReduceMoveSpeed 2e+02)))

(event Input|KeyboardEvents|T
  (params (Key :type Key%20Structure :default "None"))
  (:Pressed
    (Variables|Default|SetFreecam true))
  (:Released
    (Variables|Default|SetFreecam false)))

(fn ConstructionScript)